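; BP_Boss is a turret-style enemy that tracks the player and fires projectiles while they are within detection range.
; Tick rotates the turret body toward the player's spine_05 socket at a constant rate using RInterpToConstant.
; A one-second Delay loop from BeginPlay repeats the range check and spawns a BP_FirstPersonProjectile from the static mesh's transform, passing it the RespawnPoint actor's location.
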(event Custom|Fire%20Bullet
  ;[1 1 1] Fire Bullet
  (bind _returnvalue (Game|SpawnActorfromClass "/Game/FirstPerson/Blueprints/BP_FirstPersonProjectile.BP_FirstPersonProjectile_C" (Transformation|GetWorldTransform (Variables|Default|GetStaticMesh)) "Undefined" 0 0))
  (Variables|/Game/FirstPerson/Blueprints/BP_FirstPersonProjectile.BP_FirstPersonProjectile_C|SetRespawnPoint _returnvalue (Transformation|GetActorLocation (Variables|Default|GetRespawnPoint))))

(event EventBeginPlay
  (Utilities|FlowControl|Delay 1.0 :!label _label)
  (if (<= (Math|Vector|Distance(Vector) (Transformation|GetWorldLocation (Variables|Default|GetTurretBody)) (Transformation|GetSocketLocation (Variables|/Script/Engine.Character|GetMesh (Game|GetPlayerCharacter 0)) "spine_05")) (Variables|Default|GetDetectionDistance))
    (CallFunction|FireBullet)
    (Development|PrintString "player is near")
    (goto _label)
    (else
      (goto _label))))

(event EventTick
  (params (DeltaSeconds :type Float%20%28single-precision%29))
  (bind _returnvalue (Game|GetPlayerCharacter 0))
  (bind _turretbody (Variables|Default|GetTurretBody))
  (bind _returnvalue_2 (Transformation|GetWorldLocation _turretbody))
  (bind _mesh (Variables|/Script/Engine.Character|GetMesh _returnvalue))
  (bind _returnvalue_3 (Transformation|GetSocketLocation _mesh "spine_05"))
  (if (<= (Math|Vector|Distance(Vector) _returnvalue_2 _returnvalue_3) (Variables|Default|GetDetectionDistance))
    ;[1 1 1] LookAtPlayer
    (Transformation|SetWorldRotation _turretbody (Class|KismetMathLibrary|RInterptoConstant (Transformation|GetWorldRotation _turretbody) (Math|Rotator|FindLookatRotation _returnvalue_2 _returnvalue_3) (Utilities|Time|GetWorldDeltaSeconds) 5e+01) false false)))

(fn ConstructionScript)