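; BP_AIden is an AI-controlled pawn that follows the player character around.
; On BeginPlay it runs AI MoveTo toward the player, then waits briefly whether the move succeeds or fails.
; It then compares its Cube1 component's position with the player's capsule, polling on a delay while close and moving again once the player is far enough away.
; The loop uses looped-back Delay wires instead of Tick, with debug prints for each state.
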(event EventBeginPlay
  (bind _returnvalue (Game|GetPlayerCharacter 0))
  (AI|AIMoveTo self "0, 0, 0" _returnvalue 2e+02 false :!label _label
    (:OnSuccess
      _)
    (:OnFail
      _))
  (Utilities|FlowControl|Delay 2.0)
  (if (>= (Math|Vector|Distance(Vector) (Transformation|GetWorldLocation (Variables|Default|GetCube1)) (Transformation|GetWorldLocation (Variables|/Script/Engine.Character|GetCapsuleComponent _returnvalue))) 5e+02) :!label _label_2
    (Development|PrintString "Catching up to player")
    (goto _label)
    (else
      (Development|PrintString "Player is near")
      (Utilities|FlowControl|Delay 1.0)
      (goto _label_2))))

(event Collision|EventActorBeginOverlap
  (params (OtherActor :type Actor%20Object%20Reference)))

(event EventTick
  (params (DeltaSeconds :type Float%20%28single-precision%29)))

(fn ConstructionScript)