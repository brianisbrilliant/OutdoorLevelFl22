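; Boss actor that faces the player and fires projectiles while the player is within ActivationDistance.
; Tick rotates the Body toward the player mesh's spine_05 socket, aiming at the chest.
; A looping one-second Delay started on BeginPlay repeats the same range check and spawns a BP_FirstPersonProjectile at the BulletSpawn transform.
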(event EventBeginPlay
  ;[1 1 1] Comment
  (if (<= (Math|Vector|Distance(Vector) (Transformation|GetWorldLocation (Variables|Default|GetBody)) (Transformation|GetSocketLocation (Variables|/Script/Engine.Character|GetMesh (Game|GetPlayerCharacter 0)) "spine_05")) (Variables|Default|GetActivationDistance)) :!label _label ; If Player is near, shoot at player
    (Game|SpawnActorfromClass "/Game/FirstPerson/Blueprints/BP_FirstPersonProjectile.BP_FirstPersonProjectile_C" (Transformation|GetWorldTransform (Variables|Default|GetBulletSpawn)) "Undefined" 0 0))
  (Utilities|FlowControl|Delay 1.0)
  (goto _label))

(event EventTick
  (params (DeltaSeconds :type Float%20%28single-precision%29))
  (bind _returnvalue (Game|GetPlayerCharacter 0))
  (bind _body (Variables|Default|GetBody))
  (bind _returnvalue_2 (Transformation|GetWorldLocation _body))
  (bind _mesh (Variables|/Script/Engine.Character|GetMesh _returnvalue))
  (bind _returnvalue_3 (Transformation|GetSocketLocation _mesh "spine_05"))
  ;[1 1 1] Looking at player
  (if (<= (Math|Vector|Distance(Vector) _returnvalue_2 _returnvalue_3) (Variables|Default|GetActivationDistance)) ; if player is near, look at player
    (Transformation|SetWorldRotation (Variables|Default|GetBody) (Math|Rotator|FindLookatRotation _returnvalue_2 _returnvalue_3) false false)))

(fn ConstructionScript)